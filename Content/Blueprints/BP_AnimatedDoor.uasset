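; Animated door that slides open and closed when toggled and shows its state on a widget.
; OnToggleDoor plays or reverses a timeline according to IsDoorOpen, feeding its DoorMovement track into UpdateDoorHeight, which is defined outside this graph.
; When the timeline finishes, the widget component's WBP_TextBox is set to "Opened" or "Closed".
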(event EventBeginPlay)

(event Collision|EventActorBeginOverlap
  (params (OtherActor :type Actor%20Object%20Reference)))

(event EventTick
  (params (DeltaSeconds :type Float%20%28single-precision%29)))

(event EventOnToggleDoor
  (if (Variables|Default|GetbIsDoorOpen)
    (bind _doormovement (Timeline|TM_DoorOpenCloseTimeline Play)
      (:Update
        (Class|ArchAnimatedDoor|UpdateDoorHeight _doormovement))
      (:Finished
        (bind _aswbp_text_box (Utilities|Casting|CastToWBP_TextBox (UserInterface|GetUserWidgetObject (Variables|Default|GetStateWidgetComponent))))
        (if (Variables|Default|GetbIsDoorOpen)
          (Default|SetText _aswbp_text_box "Opened")
          (else
            (Default|SetText _aswbp_text_box "Closed")))))
    (else
      (Timeline|TM_DoorOpenCloseTimeline Reverse))))

(fn ConstructionScript)